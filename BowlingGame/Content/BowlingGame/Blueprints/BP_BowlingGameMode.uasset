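; Bowling game mode that runs the round flow through a state machine of Waiting, Ball Moving, Scoring and Game Over.
; BeginPlay caches the player pawn and pin group and creates a game-over widget.
; GMSetState toggles the pawn's shooting and updates its HUD and game-over widgets.
; On Scoring, GMCountLeftRound converts knocked pins to points and advances the round, prompting R or ending the game after three rounds.
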(event EventBeginPlay
  (bind _outactors (Actor|GetAllActorsOfClass "/Game/BowlingGame/Blueprints/BP_BowlingPlayerPawn.BP_BowlingPlayerPawn_C"))
  (Variables|Default|SetRefBowlingPawn (Utilities|Array|Get(acopy) _outactors))
  (bind _outactors_2 (Actor|GetAllActorsOfClass "/Game/BowlingGame/Blueprints/Actors/BP_BowlingPinGroup.BP_BowlingPinGroup_C"))
  (Variables|Default|SetRefPinGroup (Utilities|Array|Get(acopy) _outactors_2))
  (Variables|Default|SetICurrentRound 1)
  (bind _returnvalue (UserInterface|CreateWidget "/Game/BowlingGame/Blueprints/WBP_GameOver.WBP_GameOver_C"))
  (Variables|Default|SetGameOverWidgetRef _returnvalue))

(event EventTick
  (params (DeltaSeconds :type Float%20%28single-precision%29)))

(fn ConstructionScript)

(fn GMSetState
  (params (NewState :type E_BowlingState%20Enum :default "NewEnumerator0"))
  (bind _refbowlingpawn (Variables|Default|GetRefBowlingPawn))
  (bind _refbowlingpawn_2 (Variables|Default|GetRefBowlingPawn))
  (bind _refbowlingpawn_3 (Variables|Default|GetRefBowlingPawn))
  (bind _refbowlingpawn_4 (Variables|Default|GetRefBowlingPawn))
  (bind _gameoverwidgetref (Variables|/Game/BowlingGame/Blueprints/BP_BowlingPlayerPawn.BP_BowlingPlayerPawn_C|GetGameOverWidgetRef _refbowlingpawn))
  (bind _hudref (Variables|/Game/BowlingGame/Blueprints/BP_BowlingPlayerPawn.BP_BowlingPlayerPawn_C|GetHUDRef _refbowlingpawn_2))
  (bind _output_get (Variables|Default|SetCurrentState NewState))
  (switch Utilities|FlowControl|Switch|SwitchonE_BowlingState _output_get
    (:NewEnumerator0
      (bind _output_get_2 (Variables|Default|SetbIsGameOver false))
      (Default|SetGameOverVisibility (Variables|/Game/BowlingGame/Blueprints/BP_BowlingPlayerPawn.BP_BowlingPlayerPawn_C|GetGameOverWidgetRef (Variables|Default|GetRefBowlingPawn)) _output_get_2)
      (Variables|/Game/BowlingGame/Blueprints/BP_BowlingPlayerPawn.BP_BowlingPlayerPawn_C|SetbCanshoot _refbowlingpawn_3 true)
      (Utilities|IsValid _hudref
        (:Is%20Valid
          (Default|UpdateHUD _hudref (Variables|Default|GetICurrentRound) (Variables|Default|GetIMaxRound) (Variables|Default|GetITotalScore))
          (Default|SetPressRVisible (Variables|/Game/BowlingGame/Blueprints/BP_BowlingPlayerPawn.BP_BowlingPlayerPawn_C|GetHUDRef (Variables|Default|GetRefBowlingPawn)) false))))
    (:NewEnumerator1
      (Variables|/Game/BowlingGame/Blueprints/BP_BowlingPlayerPawn.BP_BowlingPlayerPawn_C|SetbCanshoot _refbowlingpawn_3 false))
    (:NewEnumerator2
      (Variables|/Game/BowlingGame/Blueprints/BP_BowlingPlayerPawn.BP_BowlingPlayerPawn_C|SetbCanshoot _refbowlingpawn_3 false)
      (bind _docanmoreround (CallFunction|GMCountLeftRound))
      (if _docanmoreround
        (Variables|/Game/BowlingGame/Blueprints/BP_BowlingPlayerPawn.BP_BowlingPlayerPawn_C|SetbCanshoot _refbowlingpawn_4 true)
        (Default|SetPressRVisible (Variables|/Game/BowlingGame/Blueprints/BP_BowlingPlayerPawn.BP_BowlingPlayerPawn_C|GetHUDRef _refbowlingpawn_4) true)
        (else
          (bind _output_get_3 (Variables|Default|SetCurrentState "NewEnumerator3"))
          (switch Utilities|FlowControl|Switch|SwitchonE_BowlingState _output_get_3
            (:NewEnumerator3
              (bind _output_get_4 (Variables|Default|SetbIsGameOver true))
              (Default|SetGameOverVisibility _gameoverwidgetref _output_get_4)
              (Default|SetGameOverScoreText _gameoverwidgetref))))))))

(fn GMCountLeftRound
  (bind _output_get (Variables|Default|SetIKnockedPins (Variables|/Game/BowlingGame/Blueprints/Actors/BP_BowlingPinGroup.BP_BowlingPinGroup_C|GetICountKnockDownedPin (Variables|Default|GetRefPinGroup))))
  (bind _output_get_2 (Variables|Default|SetICurrentScore (* _output_get 100)))
  (Variables|Default|SetITotalScore (+ (Variables|Default|GetITotalScore) _output_get_2))
  (if (< (Variables|Default|GetICurrentRound) 4)
    (bind _result (Math|Integer|IncrementInt (Variables|Default|GetICurrentRound))
      (:%20%20
        (Variables|Default|SetICurrentRound _result)
        (return (< (Variables|Default|GetICurrentRound) 4))))))