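; BP_BowlingPin is a bowling pin actor that can be reset to its starting placement in the bowling game.
; On BeginPlay it records its actor transform as the start transform.
; SetPinTransform zeroes the mesh's linear and angular physics velocity, teleports the actor back to that stored transform, then enables physics simulation on the static mesh.
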(event EventBeginPlay
  (Utilities|FlowControl|DoOnce false
    (:Completed
      (Variables|Default|SetBowlingPinStartTransform (Transformation|GetActorTransform)))))

(event Collision|EventActorBeginOverlap
  (params (OtherActor :type Actor%20Object%20Reference)))

(event EventTick
  (params (DeltaSeconds :type Float%20%28single-precision%29)))

(fn ConstructionScript)

(fn SetPinTransform()
  (bind _staticmesh (Variables|Default|GetStaticMesh))
  (Physics|SetPhysicsLinearVelocity _staticmesh "0, 0, 0" false "None")
  (Class|PrimitiveComponent|SetPhysicsAngularVelocityinDegrees _staticmesh "0, 0, 0" false "None")
  (Transformation|SetActorTransform (Variables|Default|GetBowlingPinStartTransform) false true)
  (Physics|SetSimulatePhysics (Variables|Default|GetStaticMesh) true))