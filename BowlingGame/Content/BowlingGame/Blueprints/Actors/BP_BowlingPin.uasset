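; Bowling pin actor that detects when it is knocked down and reports it to the pin group and player HUD.
; BeginPlay caches its start transform and group; a ball hit enables Tick and plays a one-shot, resettable sound.
; Tick flags the pin once its up vector tilts past 45 degrees via dot product, increments the group count, then stops ticking.
; PinSetTransform clears velocities and teleports it back to its start.
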(event OnComponentHit(StaticMeshComponent)
  (params (HitComponent :type Primitive%20Component%20Object%20Reference) (OtherActor :type Actor%20Object%20Reference) (OtherComp :type Primitive%20Component%20Object%20Reference) (NormalImpulse :type Vector :default "0, 0, 0") (Hit :type Hit%20Result%20Structure%20%28by%20ref%29))
  (Utilities|Casting|CastToBP_BowlingBall OtherActor)
  (Actor|Tick|SetActorTickEnabled true)
  (Utilities|FlowControl|DoOnce false
    (:Completed
      (Audio|SpawnSoundatLocation "/Game/BowlingGame/Sounds/SC_PinHitSound.SC_PinHitSound" (Transformation|GetActorLocation) "0, 0, 0" 1.0 1.0 0.0 0 0))))

(event Custom|ResetHitSoundOnce
  (Utilities|FlowControl|DoOnce false) ; enters at Reset
)

(event EventBeginPlay
  (Utilities|FlowControl|DoOnce false
    (:Completed
      (Variables|Default|SetTBowlingPinStartTransform (Transformation|GetActorTransform))
      (bind _outactors (Actor|GetAllActorsOfClass "/Game/BowlingGame/Blueprints/Actors/BP_BowlingPinGroup.BP_BowlingPinGroup_C"))
      (Variables|Default|SetRefPinGroup (Utilities|Array|Get(acopy) _outactors)))))

(event Collision|EventActorBeginOverlap
  (params (OtherActor :type Actor%20Object%20Reference)))

(event EventTick
  (params (DeltaSeconds :type Float%20%28single-precision%29))
  (CallFunction|PinSetState))

(fn ConstructionScript)

(fn PinSetTransform
  (bind _staticmeshcomponent (Variables|Default|GetStaticMeshComponent))
  (Physics|SetPhysicsLinearVelocity _staticmeshcomponent "0, 0, 0" false "None")
  (Class|PrimitiveComponent|SetPhysicsAngularVelocityinDegrees _staticmeshcomponent "0, 0, 0" false "None")
  (Transformation|SetActorTransform (Variables|Default|GetTBowlingPinStartTransform) false true)
  (Physics|SetSimulatePhysics (Variables|Default|GetStaticMeshComponent) true))

(fn IsTiltOver45
  (return (< (Math|Vector|DotProduct (Math|Vector|GetUpVector (Variables|Default|GetStaticMeshComponent)) "0.000000,0.000000,1.000000") (Math|Trig|Cos(Degrees) 45.0))))

(fn PinSetState
  (bind _refpingroup (Variables|Default|GetRefPinGroup))
  (if (not (Variables|Default|GetbKnockedDown))
    (bind _isoverthan45 (CallFunction|IsTiltOver45))
    (if _isoverthan45
      (Variables|Default|SetbKnockedDown true)
      (bind _result (Math|Integer|IncrementInt (Variables|/Game/BowlingGame/Blueprints/Actors/BP_BowlingPinGroup.BP_BowlingPinGroup_C|GetICountKnockDownedPin _refpingroup))
        (:%20%20
          (bind _output_get (Variables|/Game/BowlingGame/Blueprints/Actors/BP_BowlingPinGroup.BP_BowlingPinGroup_C|SetICountKnockDownedPin _refpingroup _result))
          (bind _asbp_bowling_player_pawn (Utilities|Casting|CastToBP_BowlingPlayerPawn (Game|Player|GetPlayerPawn 0)))
          (Default|UpdateKnockedPins (Variables|/Game/BowlingGame/Blueprints/BP_BowlingPlayerPawn.BP_BowlingPlayerPawn_C|GetHUDRef _asbp_bowling_player_pawn) _output_get)
          (Actor|Tick|SetActorTickEnabled false))))))