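; BP_BowlingPinGroup is a bowling game actor that manages the bowling pins in the level as a group.
; On BeginPlay it zeroes its knocked-down count and gathers every BP_BowlingPin in the world into an array, rather than only attached actors.
; Two functions loop over valid pins: one resets transforms, the other clears knocked-down flags, re-enables tick, zeroes the count and calls each pin's state reset.
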(event EventBeginPlay
  (Variables|Default|SetICountKnockDownedPin 0)
  (bind _outactors (Actor|GetAllActorsOfClass "/Game/BowlingGame/Blueprints/Actors/BP_BowlingPin.BP_BowlingPin_C")) ; before : get attached actors
  (for _array_element _outactors ; 각 액터들의 원본 클래스 타입들을 각각 지정해줘야 함.
    (bind _asbp_bowling_pin (Utilities|Casting|CastToBP_BowlingPin _array_element)) ; type transform: AActor -> class type actor
    (Utilities|Array|AddUnique (Variables|Default|GetBowlingPinArrays) _asbp_bowling_pin)))

(event Collision|EventActorBeginOverlap
  (params (OtherActor :type Actor%20Object%20Reference)))

(event EventTick
  (params (DeltaSeconds :type Float%20%28single-precision%29)))

(fn ConstructionScript)

(fn PinGResetPinTransform()
  (for _array_element (Variables|Default|GetBowlingPinArrays)
    (Utilities|IsValid _array_element
      (:Is%20Valid
        (Default|PinSetTransform() _array_element)))))

(fn PinGResetPinState()
  (for _array_element (Variables|Default|GetBowlingPinArrays)
    (Utilities|IsValid _array_element
      (:Is%20Valid
        (Variables|/Game/BowlingGame/Blueprints/Actors/BP_BowlingPin.BP_BowlingPin_C|SetbKnockedDown _array_element false)
        (Actor|Tick|SetActorTickEnabled _array_element true)
        (Variables|Default|SetICountKnockDownedPin 0)
        (Default|PinSetState() _array_element)))))