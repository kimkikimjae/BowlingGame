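; Physics-driven bowling ball actor that rolls with an attached rolling sound and stops at the gutter end zone.
; BallRoll applies a velocity-change impulse along the forward vector, rotated around Z by the input angle.
; On hitting BP_GutterEndZone during a specific game mode state, it zeroes velocities, fades the sound, then advances the game mode state after a delay.
; ResetBallTransform clears velocities and teleports the ball to its transform saved at BeginPlay.
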(event OnComponentHit(StaticMeshComponent)
  (params (HitComponent :type Primitive%20Component%20Object%20Reference) (OtherActor :type Actor%20Object%20Reference) (OtherComp :type Primitive%20Component%20Object%20Reference) (NormalImpulse :type Vector :default "0, 0, 0") (Hit :type Hit%20Result%20Structure%20%28by%20ref%29))
  (Utilities|Casting|CastToBP_GutterEndZone OtherActor)
  (CallFunction|StopBall)
  (bind _asbp_bowling_game_mode (Utilities|Casting|CastToBP_BowlingGameMode (Game|GetGameMode)))
  (if (Utilities|Enum|Equal(Enum) (Variables|/Game/BowlingGame/Blueprints/BP_BowlingGameMode.BP_BowlingGameMode_C|GetCurrentState _asbp_bowling_game_mode) "NewEnumerator1")
    (Utilities|FlowControl|Delay 2.0)
    (bind _asbp_bowling_game_mode_2 (Utilities|Casting|CastToBP_BowlingGameMode (Game|GetGameMode)))
    (Default|GMSetState _asbp_bowling_game_mode_2 "NewEnumerator2")))

(event EventBeginPlay
  (Variables|Default|SetBallSpawnTransform (Transformation|GetActorTransform)))

(fn ConstructionScript)

(fn BallRoll
  (params (RollingStrength :type Float%20%28double-precision%29) (InputAngle :type Float%20%28double-precision%29))
  (Physics|AddImpulse (Variables|Debug|GetStaticMeshComponent) (* RollingStrength (Math|Vector|RotateVectorAroundAxis (Transformation|GetActorForwardVector) InputAngle "0.000000,0.000000,1.000000")) "None" true)
  (bind _returnvalue (Audio|SpawnSoundAttached "/Game/BowlingGame/Sounds/SC_BallRollingSound.SC_BallRollingSound" (Variables|Debug|GetStaticMeshComponent) "None" "0, 0, 0" "0, 0, 0" "KeepRelativeOffset" false 1.0 1.0 0.0 0 0))
  (Variables|Default|SetBallRollingSound _returnvalue))

(fn ResetBallTransform
  (bind _staticmeshcomponent (Variables|Debug|GetStaticMeshComponent))
  (Physics|SetPhysicsLinearVelocity _staticmeshcomponent "0, 0, 0" false "None")
  (Class|PrimitiveComponent|SetPhysicsAngularVelocityinDegrees _staticmeshcomponent "0, 0, 0" false "None")
  (Transformation|SetActorTransform (Variables|Default|GetBallSpawnTransform) false true))

(fn StopBall
  (bind _staticmeshcomponent (Variables|Debug|GetStaticMeshComponent))
  (bind _asbp_bowling_game_mode (Utilities|Casting|CastToBP_BowlingGameMode (Game|GetGameMode)))
  (if (Utilities|Enum|Equal(Enum) (Variables|/Game/BowlingGame/Blueprints/BP_BowlingGameMode.BP_BowlingGameMode_C|GetCurrentState _asbp_bowling_game_mode) "NewEnumerator1")
    (Physics|SetPhysicsLinearVelocity _staticmeshcomponent "0, 0, 0" false "None")
    (Class|PrimitiveComponent|SetPhysicsAngularVelocityinDegrees _staticmeshcomponent "0, 0, 0" false "None")
    (bind _ballrollingsound (Variables|Default|GetBallRollingSound)
      (:then
        (Audio|Components|Audio|FadeOut _ballrollingsound 0.2 0.0 "Linear" :!class /Script/Engine.AudioComponent))
      (:else))))