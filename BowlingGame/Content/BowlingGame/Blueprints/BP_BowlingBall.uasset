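; BP_BowlingBall is the physics-driven ball actor for a bowling game, which can be rolled and reset to its starting position.
; BeginPlay caches the spawn transform.
; BallRoll applies a mass-independent impulse along world X to the static mesh, scaled by a rolling strength parameter.
; ResetBallTransform zeroes linear and angular velocity, then teleports the ball back to the cached transform.
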(event EventBeginPlay
  (Variables|Default|SetBallSpawnTransform (Transformation|GetActorTransform)))

(event Collision|EventActorBeginOverlap
  (params (OtherActor :type Actor%20Object%20Reference)))

(event EventTick
  (params (DeltaSeconds :type Float%20%28single-precision%29)))

(fn ConstructionScript)

(fn BallRoll(float)
  (params (RollingStrength :type Float%20%28double-precision%29))
  (Physics|AddImpulse (Variables|Debug|GetStaticMeshComponent) (Math|Vector|MakeVector RollingStrength 0.0 0.0) "None" true))

(fn ResetBallTransform()
  (bind _staticmeshcomponent (Variables|Debug|GetStaticMeshComponent))
  (Physics|SetPhysicsLinearVelocity _staticmeshcomponent "0, 0, 0" false "None")
  (Class|PrimitiveComponent|SetPhysicsAngularVelocityinDegrees _staticmeshcomponent "0, 0, 0" false "None")
  (Transformation|SetActorTransform (Variables|Default|GetBallSpawnTransform) false true))