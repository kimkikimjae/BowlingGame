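; Player pawn for the bowling game that creates the HUD and game-over widgets, moves sideways and launches the ball by mouse drag.
; Dragging updates the power gauge; on release, vertical drag sets roll strength and horizontal drag sets angle, then the game mode state changes.
; R restarts the whole game in game over, or resets ball, pins, state and HUD count while scoring.
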(event Input|EnhancedActionEvents|EnhancedInputActionIA_MouseClick
  (params (ActionValue :type Boolean) (ElapsedSeconds :type Float%20%28double-precision%29) (TriggeredSeconds :type Float%20%28double-precision%29) (InputAction :type Input%20Action%20Object%20Reference :default "/Game/Input/Actions/IA_MouseClick.IA_MouseClick"))
  (bind _bcanshoot (Variables|Default|GetbCanshoot))
  (bind _hudref (Variables|Default|GetHUDRef))
  (:Triggered
    (CallFunction|SetHUDDragBar))
  (:Started
    (Variables|Default|SetbIsDragging true)
    (bind _returnvalue (Class|WidgetLayoutLibrary|GetMousePositiononViewport))
    (Variables|Default|SetDragStartPos _returnvalue)
    (bind _output_get (Variables|Default|SetbShowGauge true))
    (Default|ShowPowerGauge _hudref _output_get)
    (Default|SetPowerGauge _hudref 0.0)
    (if _bcanshoot
      (bind (_returnydragstart _returnxdragstart) (CallFunction|OnMouseClickStarted()))))
  (:Completed
    (bind _output_get_2 (Variables|Default|SetbIsDragging false))
    (Default|ShowPowerGauge (Variables|Default|GetHUDRef) _output_get_2)
    (if _bcanshoot
      (bind (_returnydragend _returnxdragend) (CallFunction|OnMouseClickCompleted()))
      (bind (_outputrollingstrength _outputangle _outpower01) (CallFunction|GetRollingPower(f,F) _returnydragstart _returnydragend _returnxdragstart _returnxdragend))
      (Default|SetPowerGauge (Variables|Default|GetHUDRef) _outpower01)
      (Default|BallRoll(float,Float) (Variables|Default|GetBallRef) _outputrollingstrength _outputangle)
      (bind _asbp_bowling_game_mode (Utilities|Casting|CastToBP_BowlingGameMode (Game|GetGameMode)))
      (Default|GMSetState _asbp_bowling_game_mode "NewEnumerator1"))))

(event Input|EnhancedActionEvents|EnhancedInputActionIA_Move
  (params (ActionValue :type Vector%202D%20Structure) (ElapsedSeconds :type Float%20%28double-precision%29) (TriggeredSeconds :type Float%20%28double-precision%29) (InputAction :type Input%20Action%20Object%20Reference :default "/Game/Input/Actions/IA_Move.IA_Move"))
  (Pawn|Input|AddMovementInput (Transformation|GetActorRightVector) (.Y (Math|Vector2D|BreakVector2D ActionValue)) false))

(event Collision|EventActorBeginOverlap
  (params (OtherActor :type Actor%20Object%20Reference)))

(event EventBeginPlay
  (bind _asbp_bowling_game_mode (Utilities|Casting|CastToBP_BowlingGameMode (Game|GetGameMode)))
  (Variables|Default|SetGameModeRef _asbp_bowling_game_mode)
  (bind _returnvalue (UserInterface|CreateWidget "/Game/BowlingGame/Blueprints/WBP_MainHUD.WBP_MainHUD_C" (Game|GetPlayerController 0)))
  (bind _output_get (Variables|Default|SetHUDRef _returnvalue))
  (UserInterface|Viewport|AddtoViewport _output_get 0)
  (bind _outactors (Actor|GetAllActorsOfClass "/Game/BowlingGame/Blueprints/Actors/BP_BowlingBall.BP_BowlingBall_C"))
  (Variables|Default|SetBallRef (Utilities|Array|Get(acopy) _outactors))
  (bind _returnvalue_2 (UserInterface|CreateWidget "/Game/BowlingGame/Blueprints/WBP_GameOver.WBP_GameOver_C" (Game|GetPlayerController 0)))
  (bind _output_get_2 (Variables|Default|SetGameOverWidgetRef _returnvalue_2))
  (UserInterface|Viewport|AddtoViewport _output_get_2 0))

(event Input|KeyboardEvents|R
  (params (Key :type Key%20Structure :default "None"))
  (:Pressed
    (if (== (Variables|/Game/BowlingGame/Blueprints/BP_BowlingGameMode.BP_BowlingGameMode_C|GetCurrentState (Variables|Default|GetGameModeRef)) 3)
      (CallFunction|ResetWholeGame)
      (elif true
        (bind _currentisscoring (CallFunction|IsCurrentState==Scoring()))
        (if _currentisscoring ; Compare Enum of GameMode and block reroll by R
          (CallFunction|ResetGameRound))))))

(fn ConstructionScript)

(fn OnMouseClickStarted()
  (bind _returnvalue (Game|GetPlayerController 0))
  (bind (_locationx _locationy) (Game|Player|GetMousePosition _returnvalue))
  (bind _output_get (Variables|Default|SetXDragStart _locationx))
  (bind _output_get_2 (Variables|Default|SetYDragStart _locationy))
  (return _output_get_2 _output_get))

(fn OnMouseClickCompleted()
  (bind _returnvalue (Game|GetPlayerController 0))
  (bind (_locationx _locationy) (Game|Player|GetMousePosition _returnvalue))
  (bind _output_get (Variables|Default|SetXDragEnd _locationx))
  (bind _output_get_2 (Variables|Default|SetYDragEnd _locationy))
  (return _output_get_2 _output_get))

(fn GetRollingPower(f,F)
  (params (InputYDragStart :type Float%20%28double-precision%29) (InputYDragEnd :type Float%20%28double-precision%29) (InputXDragStart :type Float%20%28double-precision%29) (InputXDragEnd :type Float%20%28double-precision%29))
  (bind _returnvalue (Viewport|GetViewportSize))
  (bind _returnvalue_2 (- InputYDragStart InputYDragEnd))
  (bind (_x _y) (Math|Vector2D|BreakVector2D _returnvalue))
  (Utilities|FlowControl|Sequence
    (:then_0
      (if (> _returnvalue_2 0.0)
        (bind _output_get (Variables|Default|SetYDelta _returnvalue_2))))
    (:then_1
      (bind _output_get_2 (Variables|Default|SetXDelta (- InputXDragStart InputXDragEnd)))
      (bind _output_get_3 (Variables|Default|SetBowlingPower (Math|Float|Truncate (* (Math|Float|MapRangeClamped _output_get 0.0 _y 0.0 1.0) 1e+02))))
      (return (Math|Float|MapRangeClamped (Math|Conversions|ToFloat(Integer) _output_get_3) 0.0 1e+02 3e+02 1.5e+03) (* (Math|Float|MapRangeClamped _output_get_2 (* _x 0.5) (* _x -0.5) -1.0 1.0) 15.0) (Math|Float|MapRangeClamped _output_get 0.0 _y 0.0 1.0)))))

(fn ResetBallTransform()
  (Default|ResetBallTransform() (Variables|Default|GetBallRef)))

(fn ResetPinTransform()
  (bind _outactors (Actor|GetAllActorsOfClass "/Game/BowlingGame/Blueprints/Actors/BP_BowlingPinGroup.BP_BowlingPinGroup_C"))
  (bind _output_get (Variables|Default|SetRefPinGroup (Utilities|Array|Get(acopy) _outactors)))
  (Default|PinGResetPinTransform() _output_get))

(fn ResetPinState()
  (bind _outactors (Actor|GetAllActorsOfClass "/Game/BowlingGame/Blueprints/Actors/BP_BowlingPinGroup.BP_BowlingPinGroup_C"))
  (bind _output_get (Variables|Default|SetRefPinGroup (Utilities|Array|Get(acopy) _outactors)))
  (Default|PinGResetPinState() _output_get))

(fn EnableShootInput(b)
  (if (Variables|Default|GetbIsBallMoving)
    (Variables|Default|SetbIsBallMoving false)
    (else
      (Variables|Default|SetbIsBallMoving true))))

(fn IsCurrentState==Scoring()
  (bind _asbp_bowling_game_mode (Utilities|Casting|CastToBP_BowlingGameMode (Game|GetGameMode)))
  (return (Utilities|Enum|Equal(Enum) (Variables|/Game/BowlingGame/Blueprints/BP_BowlingGameMode.BP_BowlingGameMode_C|GetCurrentState _asbp_bowling_game_mode) "NewEnumerator2")))

(fn ResetCurrentGameState()
  (bind _asbp_bowling_game_mode (Utilities|Casting|CastToBP_BowlingGameMode (Game|GetGameMode)))
  (Default|GMSetState _asbp_bowling_game_mode "NewEnumerator0"))

(fn ResetHUDText
  (Default|UpdateKnockedPins (Variables|Default|GetHUDRef)))

(fn SetHUDDragBar
  (if (Variables|Default|GetbIsDragging)
    (bind _returnvalue (Class|WidgetLayoutLibrary|GetMousePositiononViewport))
    (bind _output_get (Variables|Default|SetDragCurPos _returnvalue))
    (bind _output_get_2 (Variables|Default|SetDragDelta (- _output_get (Variables|Default|GetDragStartPos))))
    (bind _output_get_3 (Variables|Default|SetCurDist (Math|Vector2D|Vector2DLength _output_get_2)))
    (Default|SetPowerGauge (Variables|Default|GetHUDRef) (Math|Float|Clamp(Float) (/ _output_get_3 (Variables|Default|GetMaxDragDist))))))

(fn ResetGameRound
  (CallFunction|ResetCurrentGameState())
  (CallFunction|ResetBallTransform())
  (CallFunction|ResetPinTransform())
  (CallFunction|ResetPinState())
  (CallFunction|ResetHUDText))

(fn ResetWholeGame
  (bind _gamemoderef (Variables|Default|GetGameModeRef))
  (Variables|/Game/BowlingGame/Blueprints/BP_BowlingGameMode.BP_BowlingGameMode_C|SetICurrentRound _gamemoderef 1)
  (Variables|/Game/BowlingGame/Blueprints/BP_BowlingGameMode.BP_BowlingGameMode_C|SetITotalScore _gamemoderef 0)
  (Default|SetPressRVisible (Variables|Default|GetHUDRef) false)
  (CallFunction|ResetGameRound))